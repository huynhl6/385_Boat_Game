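; Player-driven vehicle Blueprint for the boat_unwrapped asset, with a fuel gauge and a coin count.
; MoveForward and MoveRight axis inputs feed throttle and steering on the VehicleMovement component.
; The throttle axis event also drains Currenthealth, which serves as fuel, faster while moving forward and with no delta-time scaling or lower clamp.
; BeginPlay adds the Fuel widget to the viewport; Addcoin and Fuel functions increment coins and refuel by BarrelFuel.
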(event `self.ReceiveBeginPlay`
  (bind _returnvalue (`|CreateWidget` "/Game/UI/Fuel.Fuel_C"))
  (bind _output_get (set `self.Fuel Ref` _returnvalue))
  (`UserWidget.AddToViewport` _output_get 0))

(event `InputAxis|MoveForward`
  (params (AxisValue :type "Float (single-precision)"))
  (`WheeledVehicleMovementComponent.SetThrottleInput` (`self.VehicleMovement`) AxisValue)
  (if (>= (`WheeledVehicleMovementComponent.GetForwardSpeed` (`self.VehicleMovement`)) 0.1)
    (set `self.Currenthealth` (- (`self.Currenthealth`) 0.1))
    (else
      (set `self.Currenthealth` (- (`self.Currenthealth`) 0.01)))))

(event `InputAxis|MoveRight`
  (params (AxisValue :type "Float (single-precision)"))
  (`WheeledVehicleMovementComponent.SetSteeringInput` (`self.VehicleMovement`) AxisValue))

(fn `addcoin`
  (set `self.TotalCoins` (+ (`self.TotalCoins`) 1)))

(fn `fuel`
  (set `self.Currenthealth` (+ (`self.barrel_fuel`) (`self.Currenthealth`))))

(fn `UserConstructionScript`)